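; Actor component that acts as an inventory, holding items as identifier and description pairs and tracking one active item by index.
; AddItem rejects duplicate identifiers via ContainsItem, and SetActiveItem selects an owned item by identifier, both printing on-screen messages.
; ToggleInventory removes the open inventory widget or creates one bound to this component, adds it centre-aligned to player 0's HUD canvas and refreshes it.
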(fn `AddItem`
  (params (Identifier :type String) (Description :type String))
  (bind _result (`self.ContainsItem` Identifier))
  (if _result
    (`KismetSystemLibrary.PrintString` (`KismetStringLibrary.Concat_StrStr` "Adding " Identifier " to ItemOwner but it is already added (duplicate Identifier)."))
    (else
      (`KismetArrayLibrary.Array_Add` (`self.ContainedItems`) (make `/Game/Blueprints/Structures/ItemDescriptor` Identifier Description))
      (`KismetSystemLibrary.PrintString` (`KismetStringLibrary.Concat_StrStr` Identifier " added to item container owned by " (`KismetSystemLibrary.GetDisplayName` (`self.GetOwner`))) true true (struct :`G` 0.66 :`B` 1.0 :`A` 1.0) 4.0))))

(fn `ContainsItem`
  (params (Identifier :type String))
  (returns (Result :type Boolean) (Index :type Integer))
  (locals (DoesContainItem :type Boolean) (ItemIndex :type Integer))
  (set `local.DoesContainItem` false)
  (for (_array_element _array_index) (`self.ContainedItems`)
    (if (`KismetStringLibrary.EqualEqual_StrStr` Identifier (`.Identifier_2_22B25A0E4F7CF7CE1EB49289ACFCA884` (break `/Game/Blueprints/Structures/ItemDescriptor` _array_element)))
      (set `local.DoesContainItem` true)
      (set `local.ItemIndex` _array_index)))
  (return (`local.DoesContainItem`) (`local.ItemIndex`)))

(fn `GetActiveItem`
  (returns (Item :type "/Game/Blueprints/Structures/ItemDescriptor Structure"))
  (locals (ReturnValue :type Integer))
  (bind _activeitemindex (`self.ActiveItemIndex`))
  (set `local.ReturnValue` 0)
  (if (and (>= _activeitemindex 0) (< _activeitemindex (`KismetArrayLibrary.Array_Length` (`self.ContainedItems`))))
    (return (`|GetArrayItem` (`self.ContainedItems`) (`self.ActiveItemIndex`)))
    (else
      (return))))

(fn `SetActiveItem`
  (params (Identifier :type String))
  (bind (_result _index) (`self.ContainsItem` Identifier))
  (if _result
    (set `self.ActiveItemIndex` _index)
    (bind _item (`self.GetActiveItem`))
    (`KismetSystemLibrary.PrintString` (`KismetStringLibrary.Concat_StrStr` "Active item is " (break `/Game/Blueprints/Structures/ItemDescriptor` _item)))))

(fn `ToggleInventory`
  (returns (InventoryWindow :type "/Game/UMG/UMG_InventoryWindow Object Reference"))
  (`/Engine/EditorBlueprintResources/StandardMacros.IsValid` (`self.InventoryWindow`)
    (:`Is Valid`
      (`Widget.RemoveFromParent` (`self.InventoryWindow`))
      (set `self.InventoryWindow` null))
    (:`Is Not Valid`
      (bind _returnvalue (`|CreateWidget` "/Game/UMG/UMG_InventoryWindow.UMG_InventoryWindow_C" null self))
      (set `self.InventoryWindow` _returnvalue)
      (bind _asbp_player_controller (cast `/Game/Blueprints/BP_PlayerController` (`GameplayStatics.GetPlayerController` 0)))
      (bind _returnvalue_2 (`CanvasPanel.AddChildToCanvas` (`/Game/UMG/UMG_InGame.HUDCanvas` (`/Game/Blueprints/BP_PlayerController.HUD` _asbp_player_controller)) (`self.InventoryWindow`)))
      (`CanvasPanelSlot.SetAutoSize` _returnvalue_2 true)
      (`CanvasPanelSlot.SetAlignment` _returnvalue_2 (0.5 0.5))
      (`CanvasPanelSlot.SetAnchors` _returnvalue_2 (`self.Anchors`))
      (`/Game/UMG/UMG_InventoryWindow.Refresh` (`self.InventoryWindow`))
      (return (`self.InventoryWindow`)))))