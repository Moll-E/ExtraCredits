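; First-person player character Blueprint with look, forward/back movement, a temporary flashlight and item pickup.
; Tick aims the spotlight along control rotation and line-traces from EyesArrow to track the looked-at BP_Pickupable.
; Take passes that pickupable the player and refreshes the inventory window, which Tab toggles through ItemOwnerComponent.
; W and S presses trigger DoOnce-gated 2D footstep sound events, stopped shortly after release, with S handlers labelled wood and metal.
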(event `self.ReceiveTick`
  (params (DeltaSeconds :type "Float (single-precision)"))
  (bind _returnvalue (`SceneComponent.K2_GetComponentLocation` (`self.EyesArrow`)))
  (`|ExecutionSequence`
    (:`then_0`
      ;[1 1 1] Orient temporary flashlight to player look direction
      (`SceneComponent.K2_SetWorldRotation` (`self.FlashLightSpotLight`) (`self.GetControlRotation`) false false))
    (:`then_1`
      ;[1 1 1] The pickupable that the player is looking at.
      (bind _outhit (`KismetSystemLibrary.LineTraceSingle` _returnvalue (+ _returnvalue (* (`KismetMathLibrary.GetForwardVector` (`self.GetControlRotation`)) 500.0)) "TraceTypeQuery1"))
      (bind _asbp_pickupable (cast `/Game/Blueprints/Pickupables/BP_Pickupable` (`.HitActor` (`GameplayStatics.BreakHitResult` _outhit)))
        (:`then`
          (set `self.LookedAtPickupable` _asbp_pickupable))
        (:`CastFailed`
          (set `self.LookedAtPickupable` null))))))

(event `self.ReceiveBeginPlay`)

(event `Key|Tab`
  (params (Key :type "Key Structure"))
  ;[1 1 1] Show the player's inventory
  (:`Pressed`
    (bind _inventorywindow (`/Game/Blueprints/Components/ItemOwnerComponent.ToggleInventory` (`self.ItemOwnerComponent`)))
    (set `self.InventoryWindow` _inventorywindow)))

(event `InputAxis|MoveForwardsBackwards`
  (params (AxisValue :type "Float (single-precision)"))
  ;[1 1 1] Movement
  (`self.AddMovementInput` (* (`self.GetActorForwardVector`) AxisValue)))

(event `Key|S`
  (params (Key :type "Key Structure"))
  ;[1 1 1] FootSteps Sound Event Trigger Wood
  (:`Pressed`
    (`/Engine/EditorBlueprintResources/StandardMacros.DoOnce` false :!label _label
      (:`Completed`
        (bind _returnvalue (`FMODBlueprintStatics.PlayEvent2D` null)))))
  (:`Released`
    (`KismetSystemLibrary.Delay` 0.2)
    (`FMODBlueprintStatics.EventInstanceStop` _returnvalue)
    (goto _label :!via `Reset`)))

(event `Key|S`
  (params (Key :type "Key Structure"))
  ;[1 1 1] FootSteps Sound Event Trigger Metal
  (:`Pressed`
    (`/Engine/EditorBlueprintResources/StandardMacros.DoOnce` false :!label _label_2
      (:`Completed`
        (bind _returnvalue (`FMODBlueprintStatics.PlayEvent2D` null)))))
  (:`Released`
    (`KismetSystemLibrary.Delay` 0.2)
    (`FMODBlueprintStatics.EventInstanceStop` _returnvalue)
    (goto _label_2 :!via `Reset`)))

(event `InputAxis|LookLeftRight`
  (params (AxisValue :type "Float (single-precision)"))
  ;[1 1 1] Movement
  (`self.AddControllerYawInput` AxisValue))

(event `Key|W`
  (params (Key :type "Key Structure"))
  ;[1 1 1] FootSteps Sound Event Trigger Wood
  (:`Pressed`
    (`/Engine/EditorBlueprintResources/StandardMacros.DoOnce` false :!label _label_3
      (:`Completed`
        (bind _returnvalue (`FMODBlueprintStatics.PlayEvent2D` null)))))
  (:`Released`
    (`KismetSystemLibrary.Delay` 0.2)
    (`FMODBlueprintStatics.EventInstanceStop` _returnvalue)
    (goto _label_3 :!via `Reset`)))

(event `Key|W`
  (params (Key :type "Key Structure"))
  ;[1 1 1] FootSteps Sound Event Trigger Metal
  (:`Pressed`
    (`/Engine/EditorBlueprintResources/StandardMacros.DoOnce` false :!label _label_4
      (:`Completed`
        (bind _returnvalue (`FMODBlueprintStatics.PlayEvent2D` null)))))
  (:`Released`
    (`KismetSystemLibrary.Delay` 0.2)
    (`FMODBlueprintStatics.EventInstanceStop` _returnvalue)
    (goto _label_4 :!via `Reset`)))

(event `InputAxis|LookUpDown`
  (params (AxisValue :type "Float (single-precision)"))
  ;[1 1 1] Movement
  (`self.AddControllerPitchInput` AxisValue))

(event `InputAction|ToggleFlashlight`
  (params (Key :type "Key Structure"))
  (bind _flashlightspotlight (`self.FlashLightSpotLight`))
  ;[1 1 1] Temporary flashlight
  (:`Pressed`
    (`SceneComponent.SetHiddenInGame` _flashlightspotlight (not (`SceneComponent.bHiddenInGame` _flashlightspotlight)) false)))

(event `InputAction|Take`
  (params (Key :type "Key Structure"))
  (bind _inventorywindow (`self.InventoryWindow`))
  ;[1 1 1] Take pickupables
  (:`Pressed`
    (`/Engine/EditorBlueprintResources/StandardMacros.IsValid` (`self.LookedAtPickupable`)
      (:`Is Valid`
        (`/Game/Blueprints/Pickupables/BP_Pickupable.TakeAll` (`self.LookedAtPickupable`) self)
        (`/Engine/EditorBlueprintResources/StandardMacros.IsValid` _inventorywindow
          (:`Is Valid`
            (`/Game/UMG/UMG_InventoryWindow.Refresh` _inventorywindow)))))))

(fn `UserConstructionScript`)