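; BP_TestPickupable is a test pickup Blueprint that offers a crowbar item.
; On BeginPlay it registers the Crowbar with its ItemOwnerComponent after running the parent logic.
; Its TakeAll event passes through a DoOnce, so only the first take plays MilosDialog, AndrikDialog and CrowbarPickup together.
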(event `self.ReceiveBeginPlay`
  (`parent.ReceiveBeginPlay`)
  (`/Game/Blueprints/Components/ItemOwnerComponent.AddItem` (`self.ItemOwnerComponent`) "Crowbar" "Crowbar"))

(event `self.TakeAll`
  (params (Player :type "/Game/Blueprints/BP_PlayerCharacter Object Reference"))
  (`/Engine/EditorBlueprintResources/StandardMacros.DoOnce` false
    (:`Completed`
      (`FMODAudioComponent.Play` (`self.Milos_Dialog`))
      (`FMODAudioComponent.Play` (`self.Andrik_dialog`))
      (`FMODAudioComponent.Play` (`self.Crowbar_pickup`)))))

(fn `UserConstructionScript`
  (`parent.UserConstructionScript`))