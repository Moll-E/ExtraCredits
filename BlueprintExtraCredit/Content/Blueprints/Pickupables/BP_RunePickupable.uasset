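; Rune pickup actor that can highlight its static mesh for a rune view mode and destroys itself once its items are taken.
; BeginPlay caches the mesh's original materials.
; ActivateRuneView toggles custom depth rendering and swaps every material slot to the glow material, or restores the cached originals when deactivated.
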(event `self.ReceiveBeginPlay`
  (`parent.ReceiveBeginPlay`)
  ;[1 1 1] Hold onto mesh's original materials.
  (set `self.NormalMaterial` (`MeshComponent.GetMaterials` (`self.StaticMesh`))))

(event `self.OnItemsTaken`
  (`self.K2_DestroyActor`))

(fn `ActivateRuneView`
  (params (Active :type Boolean))
  (`PrimitiveComponent.SetRenderCustomDepth` (`self.StaticMesh`) Active)
  (if Active
    ;[1 1 1] Use glow material
    (for (_ _array_index) (`self.NormalMaterial`)
      (`PrimitiveComponent.SetMaterial` (`self.StaticMesh`) _array_index "/Game/Materials/MAT_RuneGlow.MAT_RuneGlow"))
    (else
      ;[1 1 1] Revert to original material
      (for (_array_element _array_index_2) (`self.NormalMaterial`)
        (`PrimitiveComponent.SetMaterial` (`self.StaticMesh`) _array_index_2 _array_element)))))

(fn `UserConstructionScript`
  (`parent.UserConstructionScript`))